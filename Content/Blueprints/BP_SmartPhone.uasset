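; BP_SmartPhone is the player's phone, highlighting the selected app among Kick, Twitch and YouTube on its screen widget.
; BeginPlay gathers the three WBP_Phone buttons from the LockScreen component, caches the first-person character and starts a looping half-second timer.
; While the phone is raised, CheckActiveApp reads SelectedAppIndex, sets exclusive selection flags, prints debug text and re-triggers that app's select animation.
; SelectedAppIndex is only read here, never changed.
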(event Custom|CheckActiveApp
  (if (Variables|/Game/Blueprints/BP_FirstPersonCharacter.BP_FirstPersonCharacter_C|GetPhoneRaised? (Variables|Default|GetBP_Player))
    (for _index (range 0 (- (Utilities|Array|Length (Variables|Default|Getbuttons)) 1))
      (if (== _index (Variables|Default|GetselectedAppIndex))
        (Development|PrintString (Utilities|GetDisplayName (Utilities|Array|Get(acopy) (Variables|Default|Getbuttons) _index)))
        (switch int _index
          (:0
            (Variables|Default|SetKickIsSelected? true)
            (Variables|Default|SetYouTubeIsSelected? false)
            (Variables|Default|SetTwitchIsSelected? false)
            (if (Variables|Default|GetKickIsSelected?)
              (Development|PrintString "KickisSelected")
              (bind _aswbp_phone (Utilities|Casting|CastToWBP_Phone (UserInterface|GetUserWidgetObject (Variables|Default|GetLockScreen))))
              (Default|KickSelectAnim _aswbp_phone)
              (else
                (Development|PrintString "KickisNotSelected"))))
          (:1
            (Variables|Default|SetTwitchIsSelected? true)
            (Variables|Default|SetKickIsSelected? false)
            (Variables|Default|SetYouTubeIsSelected? false)
            (if (Variables|Default|GetTwitchIsSelected?)
              (Development|PrintString "TwitchisSelected")
              (bind _aswbp_phone_2 (Utilities|Casting|CastToWBP_Phone (UserInterface|GetUserWidgetObject (Variables|Default|GetLockScreen))))
              (Default|TwitchSelectAnim _aswbp_phone_2)
              (else
                (Development|PrintString "TwitchisNotSelected"))))
          (:2
            (Variables|Default|SetYouTubeIsSelected? true)
            (Variables|Default|SetKickIsSelected? false)
            (Variables|Default|SetTwitchIsSelected? false)
            (if (Variables|Default|GetYouTubeIsSelected?)
              (Development|PrintString "YoutubeisSelected")
              (bind _aswbp_phone_3 (Utilities|Casting|CastToWBP_Phone (UserInterface|GetUserWidgetObject (Variables|Default|GetLockScreen))))
              (Default|YoutubeSelectAnim _aswbp_phone_3)
              (else
                (Development|PrintString "YoutubeisNotSelected")))))))))

(event EventBeginPlay
  (bind _lockscreen (Variables|Default|GetLockScreen))
  (bind _returnvalue (UserInterface|GetUserWidgetObject _lockscreen))
  (bind _aswbp_phone (Utilities|Casting|CastToWBP_Phone _returnvalue))
  (Utilities|FlowControl|Sequence
    (:then_0
      (Variables|Default|Setbuttons (Utilities|Array|MakeArray (Variables|/Game/UI/WBP_Phone.WBP_Phone_C|GetKick _aswbp_phone) (Variables|/Game/UI/WBP_Phone.WBP_Phone_C|GetTwitch _aswbp_phone) (Variables|/Game/UI/WBP_Phone.WBP_Phone_C|GetYoutube _aswbp_phone))))
    (:then_1
      (bind _asbp_first_person_character (Utilities|Casting|CastToBP_FirstPersonCharacter (Game|GetPlayerCharacter 0)))
      (Variables|Default|SetBP_Player _asbp_first_person_character))
    (:then_2
      (Utilities|Time|SetTimerbyFunctionName 0 "CheckActiveApp" 0.5 true))))

(fn ConstructionScript)