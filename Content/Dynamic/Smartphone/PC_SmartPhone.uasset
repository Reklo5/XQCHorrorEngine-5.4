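; Player controller that runs the first-person character's inventory UI and local inventory saves; its smartphone input event is empty.
; It swaps HUD and inventory widgets, adjusting cursor and input mode, and refreshes grids for player and container contents.
; SG_PlayerInventory slots are loaded or created, then passed to the character's server load call.
; The host loads slot 00 on BeginPlay, while clients pick a slot with number keys.
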(event Custom|SaveInventoryToSaveGame
  (params (PlayerInventory :type Array%20of%20S%20Inventory%20Content%20Structures))
  (bind _as_sg_player_inventory (Variables|Default|GetAs%20SG%20Player%20Inventory))
  (Variables|/Game/Inventory/SaveData/SG_PlayerInventory.SG_PlayerInventory_C|SetPlayerInventory _as_sg_player_inventory PlayerInventory)
  (SaveGame|SaveGametoSlot _as_sg_player_inventory (Variables|Default|GetInventorySlotName)))

(event Custom|LeaveInventoryMenu
  (bind _wb_ingamehud (Variables|Default|GetWB_IngameHUD))
  (Variables|Default|SetWB_PlayerInventory 0)
  (Variables|Default|SetbShowMouseCursor false)
  (Input|SetInputModeGameOnly self false)
  (Utilities|IsValid _wb_ingamehud
    (:Is%20Valid
      (Widget|SetVisibility _wb_ingamehud "Visible"))
    (:Is%20Not%20Valid
      (CallFunction|UIShowIngameHUD)))
  (Default|ServerCloseContainer (Variables|Default|GetAs%20BP%20First%20Person%20Character)))

(event Custom|HUD_UpdateInventoryGrid
  (params (Contents :type Array%20of%20S%20Inventory%20Content%20Structures) (PlayerInventory :type Boolean) (WorldInventory :type Boolean))
  (bind _wb_playerinventory (Variables|Default|GetWB_PlayerInventory))
  (Utilities|IsValid _wb_playerinventory
    (:Is%20Valid
      (if (UserInterface|Viewport|IsinViewport _wb_playerinventory)
        (Default|UpdateInventoryGrid (Variables|Default|GetWB_PlayerInventory) 0 PlayerInventory WorldInventory)))))

(event Custom|ContainerOpened
  (params (BP_Container :type BP%20Container%20Object%20Reference))
  (bind _wb_playerinventory (Variables|Default|GetWB_PlayerInventory))
  (bind _wb_playerinventory_2 (Variables|Default|GetWB_PlayerInventory))
  (Utilities|IsValid _wb_playerinventory
    (:Is%20Valid
      (if (UserInterface|Viewport|IsinViewport _wb_playerinventory)
        _
        (else
          (CallFunction|UIShowInventoryMenu :!label _label))))
    (:Is%20Not%20Valid
      (goto _label)))
  (Default|SetContainerWidgetsVisibility _wb_playerinventory_2 true)
  (Default|UpdateInventoryGrid _wb_playerinventory_2 (Variables|/Game/Inventory/BP_Container.BP_Container_C|GetContainerContents BP_Container) false true))

(event Input|EnhancedActionEvents|EnhancedInputActionIA_RaiseSmartPhone
  (params (ActionValue :type Boolean) (ElapsedSeconds :type Float%20%28double-precision%29) (TriggeredSeconds :type Float%20%28double-precision%29) (InputAction :type Input%20Action%20Object%20Reference :default "/Game/Dynamic/ThirdPerson/Input/Actions/IA_RaiseSmartPhone.IA_RaiseSmartPhone")))

(event EventBeginPlay
  (if (Pawn|IsLocalPlayerController)
    (CallFunction|UIShowIngameHUD)
    (if (Networking|IsServer)
      (Variables|Default|SetInventorySlotName "PlayerInventorySlot_00")
      (CallFunction|LoadInventorySaveGame)
      (Default|ServerLoadInventoryfromSaveGame (Variables|Default|GetAs%20BP%20First%20Person%20Character) (Variables|/Game/Inventory/SaveData/SG_PlayerInventory.SG_PlayerInventory_C|GetPlayerInventory (Variables|Default|GetAs%20SG%20Player%20Inventory))))))

(event EventPossess
  (params (PossessedPawn :type Pawn%20Object%20Reference))
  (bind _asbp_first_person_character (Utilities|Casting|CastToBP_FirstPersonCharacter PossessedPawn))
  (Variables|Default|SetAs%20BP%20First%20Person%20Character _asbp_first_person_character))

(event Input|KeyboardEvents|1
  (params (Key :type Key%20Structure :default "None"))
  (:Pressed
    (if (not (Networking|IsServer))
      (Variables|Default|SetInventorySlotName "PlayerInventorySlot_01")
      (CallFunction|LoadInventorySaveGame)
      (Default|ServerLoadInventoryfromSaveGame (Variables|Default|GetAs%20BP%20First%20Person%20Character) (Variables|/Game/Inventory/SaveData/SG_PlayerInventory.SG_PlayerInventory_C|GetPlayerInventory (Variables|Default|GetAs%20SG%20Player%20Inventory)))
      (Default|SetSaveSlotText (Variables|Default|GetWB_IngameHUD) "1"))))

(event Input|KeyboardEvents|2
  (params (Key :type Key%20Structure :default "None"))
  (:Pressed
    (if (not (Networking|IsServer))
      (Variables|Default|SetInventorySlotName "PlayerInventorySlot_02")
      (CallFunction|LoadInventorySaveGame)
      (Default|ServerLoadInventoryfromSaveGame (Variables|Default|GetAs%20BP%20First%20Person%20Character) (Variables|/Game/Inventory/SaveData/SG_PlayerInventory.SG_PlayerInventory_C|GetPlayerInventory (Variables|Default|GetAs%20SG%20Player%20Inventory)))
      (Default|SetSaveSlotText (Variables|Default|GetWB_IngameHUD) "2"))))

(event Input|KeyboardEvents|3
  (params (Key :type Key%20Structure :default "None"))
  (:Pressed
    (if (not (Networking|IsServer))
      (Variables|Default|SetInventorySlotName "PlayerInventorySlot_03")
      (CallFunction|LoadInventorySaveGame)
      (Default|ServerLoadInventoryfromSaveGame (Variables|Default|GetAs%20BP%20First%20Person%20Character) (Variables|/Game/Inventory/SaveData/SG_PlayerInventory.SG_PlayerInventory_C|GetPlayerInventory (Variables|Default|GetAs%20SG%20Player%20Inventory)))
      (Default|SetSaveSlotText (Variables|Default|GetWB_IngameHUD) "3"))))

(fn ConstructionScript)

(fn LoadInventorySaveGame
  (bind _returnvalue (SaveGame|DoesSaveGameExist (Variables|Default|GetInventorySlotName)))
  (if _returnvalue
    (bind _returnvalue_2 (SaveGame|LoadGamefromSlot (Variables|Default|GetInventorySlotName)))
    (bind _assg_player_inventory (Utilities|Casting|CastToSG_PlayerInventory _returnvalue_2))
    (Variables|Default|SetAs%20SG%20Player%20Inventory _assg_player_inventory)
    (else
      (bind _returnvalue_3 (SaveGame|CreateSaveGameObject "/Game/Inventory/SaveData/SG_PlayerInventory.SG_PlayerInventory_C"))
      (bind _output_get (Variables|Default|SetAs%20SG%20Player%20Inventory _returnvalue_3))
      (SaveGame|SaveGametoSlot _output_get (Variables|Default|GetInventorySlotName))))
  (return))

(fn UIShowIngameHUD
  (Utilities|IsValid (Variables|Default|GetWB_IngameHUD)
    (:Is%20Valid
      _)
    (:Is%20Not%20Valid
      (bind _returnvalue (UserInterface|CreateWidget "/Game/Inventory/Widgets/WB_IngameHUD.WB_IngameHUD_C"))
      (Variables|Default|SetWB_IngameHUD _returnvalue)))
  (UserInterface|Viewport|AddtoViewport (Variables|Default|GetWB_IngameHUD) 0)
  (return))

(fn UIShowInventoryMenu
  (bind _wb_ingamehud (Variables|Default|GetWB_IngameHUD))
  (Utilities|IsValid (Variables|Default|GetWB_PlayerInventory)
    (:Is%20Valid
      _)
    (:Is%20Not%20Valid
      (bind _returnvalue (UserInterface|CreateWidget "/Game/Inventory/Widgets/WB_PlayerInventory.WB_PlayerInventory_C"))
      (Variables|Default|SetWB_PlayerInventory _returnvalue)))
  (UserInterface|Viewport|AddtoViewport (Variables|Default|GetWB_PlayerInventory) 0)
  (Variables|Default|SetbShowMouseCursor true)
  (Input|SetInputModeGameandUI self (Variables|Default|GetWB_PlayerInventory) "DoNotLock" false false)
  (Default|UpdateInventoryGrid (Variables|Default|GetWB_PlayerInventory) (Variables|/Game/Blueprints/BP_FirstPersonCharacter.BP_FirstPersonCharacter_C|GetPlayerInventory (Variables|Default|GetAs%20BP%20First%20Person%20Character)) true false)
  (Utilities|IsValid _wb_ingamehud
    (:Is%20Valid
      (if (UserInterface|Viewport|IsinViewport _wb_ingamehud)
        (Widget|SetVisibility _wb_ingamehud "Hidden")))
    (:Is%20Not%20Valid
      _))
  (return))