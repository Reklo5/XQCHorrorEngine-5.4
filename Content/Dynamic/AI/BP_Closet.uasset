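; BP_Closet is a hiding locker that the first-person player can climb in and out of.
; Box overlap enables input and gates the hide action, which swings the door and toggles character visibility, collision and blended view target.
; While hidden, look input drives clamped pitch and yaw, applied by a self-calling MoveCamera delay loop; otherwise it passes to the character.
; AI_Search plays a separate door timeline, apparently for AI searches.
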(event OnComponentBeginOverlap(Box)
  (params (OverlappedComponent :type Primitive%20Component%20Object%20Reference) (OtherActor :type Actor%20Object%20Reference) (OtherComp :type Primitive%20Component%20Object%20Reference) (OtherBodyIndex :type Integer) (bFromSweep :type Boolean) (SweepResult :type Hit%20Result%20Structure%20%28by%20ref%29))
  ;[1 1 1] Get in and out the locker
  (bind _asbp_first_person_character (Utilities|Casting|CastToBP_FirstPersonCharacter OtherActor))
  (Variables|Default|SetCharRef _asbp_first_person_character)
  (Input|EnableInput (Game|GetPlayerController 0))
  (Utilities|FlowControl|Gate true) ; enters at Open
)

(event OnComponentEndOverlap(Box)
  (params (OverlappedComponent :type Primitive%20Component%20Object%20Reference) (OtherActor :type Actor%20Object%20Reference) (OtherComp :type Primitive%20Component%20Object%20Reference) (OtherBodyIndex :type Integer))
  (bind _returnvalue (Game|GetPlayerController 0))
  ;[1 1 1] Get in and out the locker
  (Utilities|Casting|CastToBP_FirstPersonCharacter OtherActor)
  (Input|DisableInput _returnvalue)
  (Utilities|FlowControl|Gate true) ; enters at Close
)

(event Custom|AI_Search
  (bind _doortrack (Timeline|Timeline PlayFromStart)
    (:Update
      (Transformation|SetRelativeRotation (Variables|Default|GetDoor) (Math|Rotator|MakeRotator 0.0 0.0 (Math|Float|Lerp (Variables|Default|GetCloseAngle) (Variables|Default|GetOpenAngle) _doortrack)) false false))))

(event Custom|MoveCamera
  (if (Variables|Default|GetIsHiding)
    (Transformation|SetRelativeRotation (Variables|Default|GetCamera) (Math|Rotator|MakeRotator 0.0 (* (stale Input|EnhancedActionEvents|EnhancedInputActionIA_Look _output_get) -1.0) (stale Input|EnhancedActionEvents|EnhancedInputActionIA_Look _output_get)) false false)
    (Utilities|FlowControl|Delay 0.001)
    (CallFunction|MoveCamera)))

(event Input|EnhancedActionEvents|EnhancedInputActionIA_Hiding
  (params (ActionValue :type Boolean) (ElapsedSeconds :type Float%20%28double-precision%29) (TriggeredSeconds :type Float%20%28double-precision%29) (InputAction :type Input%20Action%20Object%20Reference :default "/Game/Dynamic/ThirdPerson/Input/Actions/IA_Hiding.IA_Hiding"))
  ;[1 1 1] Get in and out the locker
  (:Started
    (Utilities|FlowControl|Gate true :!label _label
      (:Exit
        (Utilities|FlowControl|Sequence
          (:then_0
            (CallFunction|ToggleHide)
            (CallFunction|MoveCamera)
            (Utilities|FlowControl|Delay 0.2)
            (Input|EnableInput (Game|GetPlayerController 0))
            (goto _label Open))
          (:then_1
            (|OpenDoor)))))))

(event Input|EnhancedActionEvents|EnhancedInputActionIA_Look
  (params (ActionValue :type Vector%202D%20Structure) (ElapsedSeconds :type Float%20%28double-precision%29) (TriggeredSeconds :type Float%20%28double-precision%29) (InputAction :type Input%20Action%20Object%20Reference :default "/Game/Dynamic/ThirdPerson/Input/Actions/IA_Look.IA_Look"))
  (if (Variables|Default|GetIsHiding)
    (bind _output_get (Variables|Default|SetYaw (Math|Float|Clamp(Float) (+ (Variables|Default|GetYaw) (.x ActionValue)) -6e+01 6e+01)))
    (else
      (Pawn|Input|AddControllerYawInput (Variables|Default|GetCharRef) (.x ActionValue)))))

(event Input|EnhancedActionEvents|EnhancedInputActionIA_Look
  (params (ActionValue :type Vector%202D%20Structure) (ElapsedSeconds :type Float%20%28double-precision%29) (TriggeredSeconds :type Float%20%28double-precision%29) (InputAction :type Input%20Action%20Object%20Reference :default "/Game/Dynamic/ThirdPerson/Input/Actions/IA_Look.IA_Look"))
  (if (Variables|Default|GetIsHiding)
    (bind _output_get (Variables|Default|SetPitch (Math|Float|Clamp(Float) (+ (Variables|Default|GetPitch) (.y ActionValue)) -4e+01 2e+01)))
    (else
      (Pawn|Input|AddControllerPitchInput (Variables|Default|GetCharRef) (.y ActionValue)))))

(fn ConstructionScript)

(fn ToggleHide
  (bind _returnvalue (Game|GetPlayerController 0))
  (bind _charref (Variables|Default|GetCharRef))
  (if (Variables|Default|GetIsHiding)
    (Variables|Default|SetIsHiding false)
    (Rendering|SetActorHiddenInGame _charref false)
    (Collision|SetActorEnableCollision _charref true)
    (Game|Player|SetViewTargetwithBlend _returnvalue _charref 0.8 "VTBlend_Linear" 0.0 false)
    (else
      (Variables|Default|SetIsHiding true)
      (Rendering|SetActorHiddenInGame _charref true)
      (Collision|SetActorEnableCollision _charref false)
      (Game|Player|SetViewTargetwithBlend _returnvalue self 0.8 "VTBlend_Linear" 0.0 false))))