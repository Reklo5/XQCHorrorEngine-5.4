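; BP_AI is an enemy AI that spots the player and searches closets to kill a hiding player.
; Pawn sensing sets the SeeingPlayer blackboard key, while Tick eases the Legs component's yaw toward movement direction.
; CatchPlayer, called 10 seconds after BeginPlay, sphere-traces for a nearby BP_Closet and turns toward it through a short delay loop.
; It triggers the closet search, then plays a montage and kills the player if hiding.
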(event OnSeePawn(PawnSensing)
  (params (Pawn :type Pawn%20Object%20Reference))
  (if (Actor|ActorHasTag Pawn "Player")
    (AI|Components|Blackboard|SetValueasBool (AI|GetBlackboard (AI|GetAIController self)) (Utilities|Name|MakeLiteralName "SeeingPlayer") true)))

(event Custom|Catch%20Player
  (bind _returnvalue (Transformation|GetActorLocation))
  (bind (_outhits _returnvalue_2) (Collision|MultiSphereTraceByChannel _returnvalue _returnvalue 1.5e+02 "TraceTypeQuery1" false 0 "None"))
  (if _returnvalue_2
    (bind _array_element (Utilities|Array|ForEachLoopwithBreak _outhits :!label _label)
      (:LoopBody
        (bind _asbp_closet (Utilities|Casting|CastToBP_Closet (.HitActor (Collision|BreakHitResult _array_element))))
        (Variables|Default|SetClosetRef _asbp_closet)
        (goto _label Break))
      (:Completed
        (Utilities|IsValid (Variables|Default|GetClosetRef)
          (:Is%20Valid
            (Utilities|FlowControl|Sequence
              (:then_0
                (Variables|Default|SetShould%20loop? true)
                (Utilities|FlowControl|Delay 0.5)
                (Variables|Default|SetShould%20loop? false)
                (Default|AISearch (Variables|Default|GetClosetRef))
                (if (Variables|/Game/Dynamic/AI/BP_Closet.BP_Closet_C|GetIsHiding (Variables|Default|GetClosetRef))
                  (Animation|PlayAnimMontage 0 1.0 "None")
                  (Utilities|FlowControl|Delay 1.0)
                  (bind _asbp_first_person_character (Utilities|Casting|CastToBP_FirstPersonCharacter (Game|GetPlayerCharacter 0)))
                  (Default|KillPlayer _asbp_first_person_character)))
              (:then_1
                (Transformation|SetActorRotation (Math|Interpolation|RInterpTo (Transformation|GetActorRotation) (Math|Rotator|FindLookatRotation (Transformation|GetActorLocation) (Transformation|GetActorLocation (Variables|Default|GetClosetRef))) (Utilities|Time|GetWorldDeltaSeconds) 5.0))
                (Utilities|FlowControl|Delay 0.01)
                (CallFunction|LoopRot)))))))))

(event Custom|LoopRot
  (if (Variables|Default|GetShould%20loop?)
    (Transformation|SetActorRotation (Math|Interpolation|RInterpTo (Transformation|GetActorRotation) (Math|Rotator|FindLookatRotation (Transformation|GetActorLocation) (Transformation|GetActorLocation (Variables|Default|GetClosetRef))) (Utilities|Time|GetWorldDeltaSeconds) 5.0))
    (Utilities|FlowControl|Delay 0.01)
    (CallFunction|LoopRot)))

(event EventBeginPlay
  (Utilities|FlowControl|Delay 1e+01)
  (CallFunction|CatchPlayer))

(event EventTick
  (params (DeltaSeconds :type Float%20%28single-precision%29))
  (bind _returnvalue (Transformation|GetActorLocation))
  (bind _legs (Variables|Default|GetLegs))
  ;[1 1 1] Xqc Chair Rotation
  (Transformation|SetRelativeRotation _legs (Math|Rotator|MakeRotator 0.0 0.0 (Math|Interpolation|FInterpTo (.yaw (Variables|/Script/Engine.SceneComponent|GetRelativeRotation _legs)) (.yaw (Math|Rotator|FindLookatRotation _returnvalue (+ _returnvalue (Transformation|GetVelocity)))) DeltaSeconds 2.0)) false false))

(fn ConstructionScript)